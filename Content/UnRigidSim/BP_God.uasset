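; Player pawn for a rigid-body physics sandbox, with flying movement and mouse look while Move is held.
; WBP_Info triggers clearing or batch spawning of cubes and spheres at random transforms, enabling simulation once all are spawned.
; Cursor traces feed a PhysicsHandle that drags simulating bodies at adjustable distance, while non-simulating ones tilt via axis input, both with debug drawing.
; Throw launches the selected object class forward by impulse, cycled through a map.
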(event Custom|SpawnClicked_Event
  (params (Cubes :type Integer) (Spheres :type Integer))
  ;[1 1 1] User Interface
  (CallFunction|SpawnObjects (Utilities|Array|MakeArray Cubes Spheres) (Utilities|Array|MakeArray "/Game/UnRigidSim/Objects/BP_Cube.BP_Cube_C" "/Game/UnRigidSim/Objects/BP_Sphere.BP_Sphere_C")))

(event Custom|ClearClicked_Event
  ;[1 1 1] User Interface
  (for _array_element (Variables|Default|GetSpawnedObjects)
    (Actor|DestroyActor _array_element)))

(event EventBeginPlay
  (Variables|/Script/Engine.PlayerController|SetbShowMouseCursor (Game|GetPlayerController 0) true)
  (Development|ExecuteConsoleCommand "stat none 
stat fps 
stat unit" 0)
  ;[1 1 1] User Interface
  (bind _returnvalue (UserInterface|CreateWidget "/Game/UnRigidSim/WBP_Info.WBP_Info_C"))
  (bind _output_get (Variables|Default|SetInfoWidget _returnvalue))
  (UserInterface|Viewport|AddtoViewport _output_get 0)
  (EventDispatchers|AssignSpawnClicked _output_get (delegate Custom|SpawnClicked_Event))
  (EventDispatchers|AssignClearClicked _output_get (delegate Custom|ClearClicked_Event)))

(event EventTick
  (params (DeltaSeconds :type Float%20%28single-precision%29))
  (bind _physicshandle (Variables|Default|GetPhysicsHandle))
  (bind _distancetograbbedobject (Variables|Default|GetDistanceToGrabbedObject))
  (bind _physicshandle_2 (Variables|Default|GetPhysicsHandle))
  (bind _returnvalue (Class|PhysicsHandleComponent|GetGrabbedComponent _physicshandle))
  (bind _returnvalue_2 (Transformation|GetWorldRotation _returnvalue))
  (bind _returnvalue_3 (Transformation|GetWorldLocation _returnvalue))
  (bind (_roll _pitch _yaw) (Math|Rotator|BreakRotator _returnvalue_2))
  (bind _returnvalue_4 (+ _returnvalue_3 1e+02))
  ;[1 1 1] Grabbing
  (Utilities|IsValid _returnvalue
    (:Is%20Valid
      (if (Physics|IsSimulatingPhysics _returnvalue "None")
        (CallFunction|SetDistancetoObject _distancetograbbedobject)
        (bind _worldlocationatdistance (CallFunction|GetMouseLocationatDistance _distancetograbbedobject))
        (Physics|Components|PhysicsHandle|SetTargetLocation _physicshandle_2 _worldlocationatdistance)
        (Rendering|Debug|DrawDebugLine _worldlocationatdistance (Transformation|GetWorldLocation (Class|PhysicsHandleComponent|GetGrabbedComponent _physicshandle_2)) "(R=1.000000,G=0.000000,B=0.000000,A=1.000000)" 0.0 5.0)
        (else
          ;;[1 1 1] Floor Tilt
          (Transformation|SetWorldRotation _returnvalue (Math|Rotator|MakeRotator (+ _roll (Class|Actor|GetInputAxisKeyValue)) (+ _pitch (Class|Actor|GetInputAxisKeyValue)) _yaw) false false)
          (Rendering|Debug|DrawDebugArrow _returnvalue_4 (+ _returnvalue_4 "100.000000,0.000000,0.000000") 1e+02 "(R=1.000000,G=0.000000,B=0.000000,A=1.000000)" 0.0 5.0)
          (Rendering|Debug|DrawDebugArrow _returnvalue_4 (+ _returnvalue_4 "0.000000,100.000000,0.000000") 1e+02 "(R=0.000000,G=1.000000,B=0.000000,A=1.000000)" 0.0 5.0)
          (Rendering|Debug|DrawDebugArrow _returnvalue_4 (+ _returnvalue_4 "0.000000, 0,100.000000") 1e+02 "(R=0.000000,G=0.000000,B=1.000000,A=1.000000)" 0.0 5.0))))))

(event Input|ActionEvents|InputActionGrab
  (params (Key :type Key%20Structure :default "None"))
  ;[1 1 1] Grabbing
  (:Pressed
    (if (not (Variables|Default|GetIsMoving))
      (bind (_worldlocation _worldlocationatdistance) (CallFunction|GetMouseLocationatDistance 1e+05))
      (bind (_outhit _returnvalue) (Collision|LineTraceByChannel _worldlocation _worldlocationatdistance "TraceTypeQuery1" true 0 "None"))
      (if _returnvalue
        (Variables|Default|SetDistanceToGrabbedObject (.Distance (Collision|BreakHitResult _outhit)))
        (Class|PhysicsHandleComponent|GrabComponentatLocation (Variables|Default|GetPhysicsHandle) (.HitComponent (Collision|BreakHitResult _outhit)) "None" (.Location (Collision|BreakHitResult _outhit))))))
  (:Released
    (Physics|Components|PhysicsHandle|ReleaseComponent (Variables|Default|GetPhysicsHandle))))

(event Input|ActionEvents|InputActionSwitchThrowObject
  (params (Key :type Key%20Structure :default "None"))
  ;[1 1 1] Throw
  (:Pressed
    (CallFunction|SelectNextThrowObject)))

(event Input|ActionEvents|InputActionThrow
  (params (Key :type Key%20Structure :default "None"))
  ;[1 1 1] Throw
  (:Pressed
    (bind _returnvalue (Game|SpawnActorfromClass (Variables|Default|GetThrowObject) (Transformation|GetActorTransform) "AlwaysSpawn" 0 0))
    (Physics|AddImpulse (Actor|GetComponentbyClass _returnvalue "/Script/Engine.StaticMeshComponent") (* (Transformation|GetActorForwardVector) 1e+06) "None" false)))

(event Input|ActionEvents|InputActionMove
  (params (Key :type Key%20Structure :default "None"))
  (bind _returnvalue (Game|GetPlayerController 0))
  ;[1 1 1] Movement
  (:Pressed
    (Variables|Default|SetIsMoving true)
    (Variables|/Script/Engine.PlayerController|SetbShowMouseCursor _returnvalue false))
  (:Released
    (Variables|Default|SetIsMoving false)
    (Variables|/Script/Engine.PlayerController|SetbShowMouseCursor _returnvalue true)))

(event Input|AxisEvents|InputAxisMoveForward
  (params (AxisValue :type Float%20%28single-precision%29))
  ;[1 1 1] Movement
  (Pawn|Input|AddMovementInput (Transformation|GetActorForwardVector) AxisValue false))

(event Input|AxisEvents|InputAxisLookUp
  (params (AxisValue :type Float%20%28single-precision%29))
  ;[1 1 1] Movement
  (if (Variables|Default|GetIsMoving)
    (Pawn|Input|AddControllerPitchInput AxisValue)))

(event Input|AxisEvents|InputAxisMoveRight
  (params (AxisValue :type Float%20%28single-precision%29))
  ;[1 1 1] Movement
  (Pawn|Input|AddMovementInput (Transformation|GetActorRightVector) AxisValue false))

(event Input|AxisEvents|InputAxisMoveUp
  (params (AxisValue :type Float%20%28single-precision%29))
  ;[1 1 1] Movement
  (Pawn|Input|AddMovementInput (Transformation|GetActorUpVector) AxisValue false))

(event Input|AxisEvents|InputAxisTurn
  (params (AxisValue :type Float%20%28single-precision%29))
  ;[1 1 1] Movement
  (if (Variables|Default|GetIsMoving)
    (Pawn|Input|AddControllerYawInput AxisValue)))

(fn ConstructionScript)

(fn GetMouseLocationatDistance
  (params (Distance :type Float%20%28single-precision%29))
  (bind _returnvalue (Game|GetPlayerController 0))
  (bind (_worldlocation _worlddirection) (Game|Player|ConvertMouseLocationToWorldSpace _returnvalue))
  (return _worldlocation (+ _worldlocation (* _worlddirection Distance))))

(fn SelectNextThrowObject
  (bind _throwobjects (Variables|Default|GetThrowObjects))
  (bind _keys (Utilities|Map|Keys _throwobjects))
  (bind _output_get (LocalVariables|SetSwitchedIndex (Class|KismetMathLibrary|Wrap (+ (Utilities|Array|FindItem _keys (Variables|Default|GetThrowObject)) 1) -1 (- (Utilities|Map|Length _throwobjects) 1)))) ; Temporary variable to prevent overwriting index
  (Variables|Default|SetThrowObject (Utilities|Array|Get(acopy) _keys _output_get))
  (bind _values (Utilities|Map|Values (Variables|Default|GetThrowObjects)))
  (Variables|/Game/UnRigidSim/WBP_Info.WBP_Info_C|SetSelectedObject (Variables|Default|GetInfoWidget) (Utilities|Array|Get(acopy) _values (LocalVariables|GetSwitchedIndex))))

(fn SetDistancetoObject
  (params (Distance :type Float%20%28single-precision%29%20%28by%20ref%29))
  (Variables|Default|SetDistanceToGrabbedObject (+ Distance (* (Class|Actor|GetInputAxisKeyValue) 5e+01)))
  (return))

(fn SpawnObjects
  (params (Counts :type Array%20of%20Integers) (Classes :type Array%20of%20Actor%20Class%20References))
  (bind _spawned (LocalVariables|GetSpawned))
  (bind _total (CallFunction|SumOfArray Counts))
  (LocalVariables|SetTotal _total)
  ;[1 1 1] Each class
  (for _index (range 0 (- (Utilities|Array|Length Counts) 1))
    ;[1 1 1] Spawn count of current class (with disabled simulation)
    (bind _output_get (LocalVariables|SetRemaining (Utilities|Array|Get(acopy) Counts _index)))
    (while (> _output_get 0)
      (bind _returnvalue (CallFunction|GetRandomSpawnTransform "0.000000,0,1000.000000" (LocalVariables|GetTotal)))
      (bind _returnvalue_2 (Game|SpawnActorfromClass (Utilities|Array|Get(acopy) Classes _index) _returnvalue "AdjustIfPossibleButAlwaysSpawn" 0 0))
      (Utilities|Array|Add (Variables|Default|GetSpawnedObjects) _returnvalue_2)
      (Physics|SetSimulatePhysics (Actor|GetComponentbyClass _returnvalue_2 "/Script/Engine.StaticMeshComponent") false)
      (Utilities|Array|Add (LocalVariables|GetSpawned) (Actor|GetComponentbyClass _returnvalue_2 "/Script/Engine.StaticMeshComponent"))
      (Math|Integer|DecrementInt (LocalVariables|GetRemaining))))
  ;[1 1 1] Enable simulation on all
  (for _array_element _spawned
    (Physics|SetSimulatePhysics _array_element true))
  (Development|PrintString (Utilities|String|Append (Utilities|String|ToString(Integer) (Utilities|Array|Length _spawned)) " spawned")))

(fn GetRandomSpawnTransform
  (params (AreaCenter :type Vector :default "0.000000,0,1000.000000") (Total%20Count :type Integer))
  (return (Math|Transform|MakeTransform (Math|Random|RandomPointinBoundingBox AreaCenter (Math|Vector|MakeVector 1e+03 1e+03 (Math|Conversions|ToFloat(Integer) (* Total%20Count 5)))) (Math|Random|RandomRotator true))))

(fn SumOfArray
  (params (Values :type Array%20of%20Integers))
  (for _array_element Values
    (bind _output_get (LocalVariables|SetSum (+ _array_element (LocalVariables|GetSum))))
    (return _output_get)))